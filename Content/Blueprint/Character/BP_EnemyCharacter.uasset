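; Enemy character that supplies wander and patrol destinations and handles its own death.
; Patrollers start at the nearest PatrolPath spline point and cycle through points in a loop.
; Wander points come from random navmesh locations, retried recursively, then stored as Destination with a debug sphere.
; On death it plays a montage and material effect, hides, line-traces to place a pickup nearby, then destroys its weapon and itself.
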(event EventBeginPlay
  (|CallParentFunction)
  (if (Variables|Default|GetIsPatroller)
    (bind _index (CallFunction|GetClosestPatrolPath))
    (Variables|Default|SetPatrolIndex _index)))

(event Collision|EventActorBeginOverlap
  (params (OtherActor :type Actor%20Object%20Reference))
  (|CallParentFunction OtherActor) ; This node is disabled and will not be called.\nDrag off pins to build functionality.
)

(event EventTick
  (params (DeltaSeconds :type Float%20%28single-precision%29))
  (|CallParentFunction DeltaSeconds))

(event EventCharacterDie
  (Animation|PlayAnimMontage (Variables|Default|GetAnim%20Montage%20Die) 1.0 "None")
  (Utilities|FlowControl|Delay 1.0)
  (CallFunction|PlayMaterialEffect "(R=0.052083,G=0.001462,B=0.000000,A=1.000000)")
  (Utilities|FlowControl|Delay 1.0)
  (Rendering|SetVisibility (Variables|Character|GetMesh) false false)
  (CallFunction|SpawnPickup)
  (Actor|DestroyActor (Variables|Default|GetCurrentWeapon))
  (Actor|DestroyActor))

(fn ConstructionScript
  (|CallParentFunction))

(fn SetDestination
  (params (Destination :type Vector))
  (bind _output_get (Variables|Default|SetDestination Destination))
  (Rendering|Debug|DrawDebugSphere _output_get 1e+01 12 "(R=0.000000,G=1.000000,B=0.045144,A=1.000000)" 1e+01 2.0))

(fn GetNextNavPoint
  (bind (_randomlocation _returnvalue) (Class|NavigationSystemV1|GetRandomLocationinNavigableRadius (Transformation|GetActorLocation) 3e+02 0 0))
  (if _returnvalue
    (CallFunction|SetDestination _randomlocation)
    (else
      (CallFunction|GetNextNavPoint))))

(fn SpawnPickup
  (bind _returnvalue (Transformation|GetActorLocation))
  (bind (_outhit _returnvalue_2) (Collision|LineTraceForObjects (+ _returnvalue "0.000000,0.000000,1000.000000") (- _returnvalue "0.000000,0.000000,1000.000000") (Utilities|Array|MakeArray "ObjectTypeQuery1" "ObjectTypeQuery2") false 0 "Persistent"))
  (if _returnvalue_2
    (bind _randomlocation (Class|NavigationSystemV1|GetRandomLocationinNavigableRadius (.Location (Collision|BreakHitResult _outhit)) 5e+01 0 0))
    (Game|SpawnActorfromClass (Variables|Default|GetPickupClass) (Math|Conversions|ToTransform(Vector) (+ _randomlocation "0.000000,0.000000,10.000000")) "Undefined" 0 0)))

(fn GetClosestPatrolPath
  (bind _patrolpath (Variables|Setting|GetPatrolPath))
  (Utilities|IsValid _patrolpath
    (:Is%20Valid
      (return (Math|Float|Floor (Class|SplineComponent|FindInputKeyClosesttoWorldLocation (Variables|/Game/Blueprint/AI/AICrowl/BP_PatrolPath.BP_PatrolPath_C|GetPatrolPath _patrolpath) (Transformation|GetActorLocation)))))
    (:Is%20Not%20Valid
      (return 0))))

(fn GetNextPatrolPath
  (bind _patrolpath (Variables|Setting|GetPatrolPath))
  (bind _patrolpath_2 (Variables|/Game/Blueprint/AI/AICrowl/BP_PatrolPath.BP_PatrolPath_C|GetPatrolPath _patrolpath))
  (bind _result (Math|Integer|IncrementInt (Variables|Default|GetPatrolIndex))
    (:%20%20
      (if (>= _result (Spline|GetNumberOfSplinePoints _patrolpath_2))
        (bind _output_get (Variables|Default|SetPatrolIndex 0))
        (return (Spline|GetLocationatSplinePoint _patrolpath_2 _output_get "World"))
        (else
          (bind _output_get_2 (Variables|Default|SetPatrolIndex _result))
          (return (Spline|GetLocationatSplinePoint _patrolpath_2 _output_get_2 "World")))))))