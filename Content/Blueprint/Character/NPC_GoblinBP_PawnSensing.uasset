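; Goblin NPC Blueprint that patrols nav points and uses PawnSensing to spot, chase and melee-attack pawns.
; While alive, delayed Tick logic moves it toward its target, attacking on arrival, or toward its destination, picking a new nav point on success or abort.
; Seeing a pawn sets the target and losing line of sight clears it.
; Loud noises redirect the destination and draw a debug sphere.
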(event OnSeePawn(MyPawnSensing)
  (params (Pawn :type Pawn%20Object%20Reference))
  (Variables|Default|SetTargetPawn Pawn))

(event OnHearNoise(MyPawnSensing)
  (params (Instigator :type Pawn%20Object%20Reference) (Location :type Vector%20%28by%20ref%29 :default "0, 0, 0") (Volume :type Float%20%28single-precision%29))
  (if (> Volume 3e+02)
    (bind _output_get (Variables|Default|SetDestination Location))
    (Rendering|Debug|DrawDebugSphere _output_get 1e+01 12 "(R=1.000000,G=0.962178,B=0.026111,A=1.000000)" 1e+01 2.0)))

(event EventBeginPlay
  (|CallParentFunction)
  (CallFunction|GetNextNavPoint))

(event Collision|EventActorBeginOverlap
  (params (OtherActor :type Actor%20Object%20Reference))
  (|CallParentFunction OtherActor) ; This node is disabled and will not be called.\nDrag off pins to build functionality.
)

(event EventTick
  (params (DeltaSeconds :type Float%20%28single-precision%29))
  (bind _self self)
  (|CallParentFunction DeltaSeconds)
  (Utilities|FlowControl|Delay 0.2)
  (if (CallFunction|IsAlive)
    (Utilities|FlowControl|Sequence
      (:then_0
        (Utilities|IsValid (Variables|Default|GetTargetPawn)
          (:Is%20Valid
            (AI|AIMoveTo _self "0, 0, 0" (Variables|Default|GetTargetPawn) 3e+01 true
              (:OnSuccess
                (CallFunction|DoMeleeAttack))))
          (:Is%20Not%20Valid
            (bind _movementresult (AI|AIMoveTo _self (Variables|Default|GetDestination) 0 3e+01 true)
              (:then
                (switch Utilities|FlowControl|Switch|SwitchonEPathFollowingResult _movementresult
                  (:Success
                    _)
                  (:Aborted
                    (Utilities|FlowControl|Delay 1.0)
                    (switch Utilities|FlowControl|Switch|SwitchonEPathFollowingResult _movementresult
                      (:Aborted
                        _))))
                (CallFunction|GetNextNavPoint))))))
      (:then_1
        (Utilities|IsValid (Variables|Default|GetTargetPawn)
          (:Is%20Valid
            (if (not (Class|MyPawnSensingComponent|HasLineOfSightto (Variables|Default|GetMyPawnSensing) (Variables|Default|GetTargetPawn)))
              (Variables|Default|SetTargetPawn 0))))))))

(fn ConstructionScript
  (|CallParentFunction))