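; Goblin NPC Blueprint that patrols in an endless loop along a spline path.
; On BeginPlay it copies the world location of each PatrolPath spline point into an array.
; WalkToNextPoint picks the next index, wrapping to the first, runs AI Move To and calls itself again on success.
; A failed move has no handler, so the patrol does not continue from it.
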(event Custom|WalkToNextPoint
  (CallFunction|SetNextPatrolPoint)
  (AI|AIMoveTo self (Utilities|Array|Get(acopy) (Variables|Default|GetPatrolPoint) (Variables|Default|GetTargetPatrolIndex)) 0 5.0 false
    (:OnSuccess
      (Utilities|FlowControl|Sequence
        (:then_0
          (Variables|Default|SetCurrentPatrolIndex (Variables|Default|GetTargetPatrolIndex)))
        (:then_1
          (CallFunction|WalktoNextPoint))))))

(event EventBeginPlay
  (|CallParentFunction)
  (CallFunction|InitialPatrolPathOld)
  (CallFunction|WalktoNextPoint))

(event Collision|EventActorBeginOverlap
  (params (OtherActor :type Actor%20Object%20Reference))
  (|CallParentFunction OtherActor) ; This node is disabled and will not be called.\nDrag off pins to build functionality.
)

(event EventTick
  (params (DeltaSeconds :type Float%20%28single-precision%29)))

(fn ConstructionScript
  (|CallParentFunction))

(fn InitialPatrolPathOld
  (bind _self self)
  (bind _patrolpath (Variables|Default|GetPatrolPath _self))
  (bind _patrolpath_2 (Variables|/Game/Blueprint/AI/AICrowl/BP_PatrolPath.BP_PatrolPath_C|GetPatrolPath _patrolpath))
  (for _index (range 0 (- (Spline|GetNumberOfSplinePoints _patrolpath_2) 1))
    (Utilities|Array|Add (Variables|Default|GetPatrolPoint) (Spline|GetLocationatSplinePoint _patrolpath_2 _index "World")))
  (Variables|Default|SetCurrentPatrolIndex 0))

(fn SetNextPatrolPoint
  (if (< (Variables|Default|GetCurrentPatrolIndex) (- (Utilities|Array|Length (Variables|Default|GetPatrolPoint)) 1))
    (Variables|Default|SetTargetPatrolIndex (+ (Variables|Default|GetCurrentPatrolIndex) 1))
    (else
      (Variables|Default|SetTargetPatrolIndex 0))))