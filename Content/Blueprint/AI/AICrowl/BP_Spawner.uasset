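; Enemy spawner actor that spawns waves of BP_EnemyCharacter over a set number of rounds.
; A delayed Tick checks IsAllDead, spawning and decrementing Rounds, or calling RoundsFinish once at zero; GoblinFactory also runs before the round check.
; GoblinFactory clears the list, line-traces for ground and spawns at random navigable points, with debug drawing.
; Otherwise, Tick removes entries reporting IsAlive, not dead ones, from SpawnedEnemies.
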(event EventBeginPlay)

(event Collision|EventActorBeginOverlap
  (params (OtherActor :type Actor%20Object%20Reference)))

(event EventTick
  (params (DeltaSeconds :type Float%20%28single-precision%29))
  (bind _spawnedenemies (Variables|Default|GetSpawnedEnemies))
  (Utilities|FlowControl|Delay 0.2)
  (if (Variables|Default|GetIsAllDead)
    (CallFunction|GoblinFactory)
    (if (> (Variables|Default|GetRounds) 0)
      (CallFunction|GoblinFactory)
      (Variables|Default|SetRounds (- (Variables|Default|GetRounds) 1))
      (else
        (Utilities|FlowControl|DoOnce false
          (:Completed
            (Default|CallRoundsFinish)))))
    (elif (> (Utilities|Array|Length _spawnedenemies) 0)
      (for _array_element _spawnedenemies
        (if (Default|IsAlive _array_element)
          (Utilities|Array|RemoveItem (Variables|Default|GetSpawnedEnemies) _array_element))))))

(fn ConstructionScript)

(fn GoblinFactory
  (bind _returnvalue (Transformation|GetActorLocation))
  (bind _returnvalue_2 (Transformation|GetActorTransform))
  (bind _num (Variables|Default|GetNum))
  (Utilities|Array|Clear (Variables|Default|GetSpawnedEnemies))
  (if (> _num 0)
    (for _index (range 0 (- _num 1))
      (bind (_outhit _returnvalue_3) (Collision|LineTraceForObjects (+ _returnvalue "0.000000,0.000000,1000.000000") (- _returnvalue "0.000000,0.000000,1000.000000") (Utilities|Array|MakeArray "ObjectTypeQuery1" "ObjectTypeQuery2") false 0 "Persistent"))
      (if _returnvalue_3
        (bind _randomlocation (Class|NavigationSystemV1|GetRandomLocationinNavigableRadius (.Location (Collision|BreakHitResult _outhit)) (Variables|Default|GetRadius) 0 0))
        (Rendering|Debug|DrawDebugSphere _randomlocation 3e+01 4 "(R=1.000000,G=0.030093,B=0.010197,A=1.000000)" 5.0 2.0)
        (bind _returnvalue_4 (Game|SpawnActorfromClass (Variables|Default|GetEnemyClass) (Math|Transform|MakeTransform _randomlocation (.rotation _returnvalue_2) (.scale _returnvalue_2)) "Undefined" self 0))
        (bind _asbp_enemy_character (Utilities|Casting|CastToBP_EnemyCharacter _returnvalue_4))
        (Utilities|Array|Add (Variables|Default|GetSpawnedEnemies) _asbp_enemy_character)))))